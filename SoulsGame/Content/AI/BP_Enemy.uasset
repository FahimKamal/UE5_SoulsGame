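; Sword-wielding enemy character with a health bar widget, a montage attack and ragdoll death.
; BeginSwordTrace and EndSwordTrace toggle a looping timer that sphere-traces pawns between two sword points, with a DoOnce and short delay throttling damage.
; Incoming damage is passed as a negative change to the BPCStats component, which receives the health bar on BeginPlay.
; Die disables movement, enables mesh physics and stops further trace damage.
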(event `self.ReceiveBeginPlay`
  (bind _aswb_enemy_health (cast `/Game/UI/WB_EnemyHealth` (`WidgetComponent.GetWidget` (`self.Widget`))))
  (`/Game/Blueprints/BPC_Stats.Set Health Progress Bar` (`self.BPC_Stats`) (`/Game/UI/WB_EnemyHealth.HealthBar` _aswb_enemy_health)))

(event `/Game/Blueprints/BPI_Damage.End Sword Trace`
  ;[0.2865 0.3221 0.4219] Sword Traces
  (if (`KismetSystemLibrary.K2_IsValidTimerHandle` (stale `/Game/Blueprints/BPI_Damage.Begin Sword Trace` _returnvalue))
    (`KismetSystemLibrary.K2_ClearAndInvalidateTimerHandle` (stale `/Game/Blueprints/BPI_Damage.Begin Sword Trace` _returnvalue))))

(event `/Game/Blueprints/BPI_Damage.Begin Sword Trace`
  ;[0.2865 0.3221 0.4219] Sword Traces
  (bind _returnvalue (`KismetSystemLibrary.K2_SetTimerDelegate` (delegate `Damage Trace`) 0.01 true)))

(event `Damage Trace`
  ;[0.2865 0.3221 0.4219] Sword Traces
  (if (not (`self.isDead?`))
    (bind (_outhit _returnvalue) (`KismetSystemLibrary.SphereTraceSingleForObjects` :`Start` (`SceneComponent.K2_GetComponentLocation` (`self.Start Sword Trace Pos`)) :`End` (`SceneComponent.K2_GetComponentLocation` (`self.End Sword Trace Pos`)) :`Radius` 25.0 :`ObjectTypes` (`|MakeArray` "ObjectTypeQuery3" :!type "EObjectTypeQuery Enum") :`DrawDebugType` "ForOneFrame"))
    (if _returnvalue
      (`/Engine/EditorBlueprintResources/StandardMacros.DoOnce` false :!label _label
        (:`Completed`
          (`GameplayStatics.ApplyDamage` (`.HitActor` (`GameplayStatics.BreakHitResult` _outhit)) (`self.Sword  Damage`))
          (`KismetSystemLibrary.Delay` 0.3)
          (goto _label :!via `Reset`))))))

(event `self.ReceiveAnyDamage`
  (params (Damage :type "Float (single-precision)") (DamageType :type "DamageType Object Reference") (InstigatedBy :type "Controller Object Reference") (DamageCauser :type "Actor Object Reference"))
  ;[0.01096 0.01161 0.0137] Damage Enemy
  (`/Game/Blueprints/BPC_Stats.Increase Value` (`self.BPC_Stats`) "NewEnumerator0" (* Damage -1.0)))

(event `/Game/Blueprints/BPI_Damage.Die`
  (`CharacterMovementComponent.DisableMovement` (`self.CharacterMovement`))
  (`PrimitiveComponent.SetSimulatePhysics` (`self.Mesh`) true)
  (set `self.isDead?` true))

(fn `Sword Attack`
  (returns (Duration :type "Float (double-precision)"))
  (bind _returnvalue (`self.PlayAnimMontage` "/Game/Characters/Souls/Combat/SwordAttackCombo_Montage.SwordAttackCombo_Montage"))
  (return _returnvalue))

(fn `UserConstructionScript`)